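; GA_Player_Heal is a player gameplay ability that slows the avatar character while the heal plays.
; On activation it lowers the character's CharacterMovement max walk speed, and on end it restores a hardcoded normal speed.
; The previous speed is cached in TempSpeed but never used for the restore.
; The graph contains no healing, montage, or EndAbility call.
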(event Ability|EventActivateAbility
  ;[0.15 0.15 0.15 0.5] 再生中の移動速度を変える
  (bind _ascharacter (Utilities|Casting|CastToCharacter (Ability|GetAvatarActorfromActorInfo)))
  (Variables|Default|SetTempSpeed (Variables|/Script/Engine.CharacterMovementComponent|GetMaxWalkSpeed (Variables|/Script/Engine.Character|GetCharacterMovement _ascharacter)))
  (Variables|/Script/Engine.CharacterMovementComponent|SetMaxWalkSpeed (Variables|/Script/Engine.Character|GetCharacterMovement _ascharacter) 1e+02))

(event Ability|EventOnEndAbility
  (params (bWasCancelled :type Boolean))
  ;[0.15 0.15 0.15 0.5] 戻す
  (bind _ascharacter (Utilities|Casting|CastToCharacter (Ability|GetAvatarActorfromActorInfo)))
  (Variables|/Script/Engine.CharacterMovementComponent|SetMaxWalkSpeed (Variables|/Script/Engine.Character|GetCharacterMovement _ascharacter) 3.8e+02))