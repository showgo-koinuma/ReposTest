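; BP_DamageNiagara is a monster ability cue actor that plays a Niagara effect which damages the player.
; On BeginPlay it registers itself as the Niagara BPCallBack export target and destroys itself after NiagaraDuration.
; When particle data arrives, it casts its owner to MonsterCharacter and calls DealDamage on player 0.
; A system-finished binding sits unused, noted as having timing problems.
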(event EventBeginPlay
  (Class|NiagaraComponent|SetVariableObject (Variables|Default|GetDamageNiagara) "BPCallBack" self)
  (Utilities|FlowControl|Delay (Variables|Default|GetNiagaraDuration))
  (Actor|DestroyActor))

(event EventParticleData
  (params (Data :type Array%20of%20Basic%20Particle%20Data%20Structures) (NiagaraSystem :type Niagara%20System%20Object%20Reference) (SimulationPositionOffset :type Vector%20%28by%20ref%29 :default "0, 0, 0"))
  (bind _asmonster_character (Utilities|Casting|CastToMonsterCharacter (Components|GetOwner)))
  (Class|MonsterCharacter|DealDamage _asmonster_character (Game|GetPlayerCharacter 0)))

(fn ConstructionScript)