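; Player character Blueprint that sets up the player's starting state at BeginPlay, applying a zero pitch input and granting heal items through PlayerItemManager.
; Every Tick, it nudges the movement component's updated component diagonally out and back with sweep enabled.
; Pressing Q prints the names of the active abilities from CustomAbilitySystemComponent for debugging.
; A PlayMontage node on the mesh is left unconnected and never runs.
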(event EventTick
  (params (DeltaSeconds :type Float%20%28single-precision%29))
  (bind _returnvalue (Transformation|GetActorRotation))
  (bind _charactermovement (Variables|Character|GetCharacterMovement))
  (Class|MovementComponent|MoveUpdatedComponent _charactermovement "1.000000,1.000000,0.000000" _returnvalue true)
  (Class|MovementComponent|MoveUpdatedComponent _charactermovement "-1.000000,-1.000000,0.000000" _returnvalue true))

(event EventBeginPlay
  ;[0.15 0.15 0.15 0.5] ゲーム開始時の初期の視点
  (Pawn|Input|AddControllerPitchInput 0.0)
  ;[0.15 0.15 0.15 0.5] 初期アイテムを追加
  (Class|PlayerItemManager|AddItem (Variables|Default|GetPlayerItemManager) "/Game/Blueprint/Item/BP_Item_Heal.BP_Item_Heal_C" 10))

(event Input|KeyboardEvents|Q
  (params (Key :type Key%20Structure :default "None"))
  (:Pressed
    (for _array_element (Class|CustomAbilitySystemComponent|GetActiveAbilities (Variables|Default|GetCustomAbilitySystemComponent))
      (Development|PrintString (Utilities|GetObjectName _array_element)))))

(fn ConstructionScript)