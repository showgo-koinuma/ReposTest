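; Anim notify that spawns a DamageNiagara actor at the frame it is placed on in an animation.
; The spawn location is a named socket on the animated mesh plus an offset added directly in world space.
; The rotation combines the mesh's world rotation with a relative rotator, independent of the socket's rotation.
; The mesh's owning actor becomes the owner of the spawned actor.
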(fn ReceivedNotify
  (params (MeshComp :type Skeletal%20Mesh%20Component%20Object%20Reference) (Animation :type Anim%20Sequence%20Base%20Object%20Reference) (EventReference :type Anim%20Notify%20Event%20Reference%20Structure%20%28by%20ref%29))
  (Game|SpawnActorfromClass (Variables|Default|GetDamageNiagara) (Math|Transform|MakeTransform (+ (Transformation|GetSocketLocation MeshComp (Variables|Default|GetIn%20Socket%20Name)) (Variables|Default|GetOffsetFromSocket)) (Math|Rotator|CombineRotators (Transformation|GetWorldRotation MeshComp) (Variables|Default|GetRelativeRotationFromMesh)) "1.000000,1.000000,1.000000") "Undefined" "MultiplyWithRoot" (Components|GetOwner MeshComp) 0)
  (return false))