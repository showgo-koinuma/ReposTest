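; Animation notify that spawns a configurable Niagara system at a named socket on the animated mesh.
; When AttachToMesh is set, it spawns the system attached to that socket with auto-destroy.
; Otherwise it spawns it in world space at the socket location plus an offset, rotated by the mesh's world rotation combined with a relative rotation.
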(fn ReceivedNotify
  (params (MeshComp :type Skeletal%20Mesh%20Component%20Object%20Reference) (Animation :type Anim%20Sequence%20Base%20Object%20Reference) (EventReference :type Anim%20Notify%20Event%20Reference%20Structure%20%28by%20ref%29))
  (bind _in_socket_name (Variables|Default|GetIn%20Socket%20Name))
  (if (Variables|Default|GetAttachToMesh)
    (Niagara|SpawnSystemAttached (Variables|Default|GetSpawnNiagara) MeshComp _in_socket_name "0, 0, 0" "0, 0, 0" "KeepRelativeOffset" true)
    (else
      (Niagara|SpawnSystematLocation (Variables|Default|GetSpawnNiagara) (+ (Transformation|GetSocketLocation MeshComp _in_socket_name) (Variables|Default|GetOffsetFromSocket)) (Math|Rotator|CombineRotators (Transformation|GetWorldRotation MeshComp) (Variables|Default|GetRelativeRotationFromMesh)))))
  (return false))