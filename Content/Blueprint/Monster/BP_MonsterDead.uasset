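; BP_MonsterDead is a dead-monster actor that plays a death animation and provides the exit from gameplay to the title level.
; On BeginPlay it plays AM_Mons_Dead, then on completion replays it from the Cut section at zero play rate to hold that pose.
; EndInGame shows the loading widget, then loads and opens TitleLevel.
; An unconnected branch would play the quest-clear sequence relative to the mesh transform.
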(event Custom|EndInGame
  (bind _returnvalue (UserInterface|CreateWidget "/Game/Blueprint/WidgetBP/Title/WBP_Loading.WBP_Loading_C"))
  (UserInterface|Viewport|AddtoViewport _returnvalue 0)
  (Class|GameplayStatics|LoadStreamLevelbySoftObjectPtr "/Game/Levels/TitleLevel.TitleLevel" false false)
  (Game|OpenLevel(byObjectReference) "/Game/Levels/TitleLevel.TitleLevel"))

(event EventBeginPlay
  (bind _skeletalmesh (Variables|Default|GetSkeletalMesh))
  (Utilities|FlowControl|Sequence
    (:then_1
      (Animation|Montage|PlayMontage _skeletalmesh "/Game/Characters/Monster/Animation/Montage/AM_Mons_Dead.AM_Mons_Dead" 1.0 0.0 "Default"
        (:OnCompleted
          (Animation|Montage|PlayMontage _skeletalmesh "/Game/Characters/Monster/Animation/Montage/AM_Mons_Dead.AM_Mons_Dead" 0.0 0.0 "Cut"))))))

(fn ConstructionScript)